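; BP_SettingsSaveGame is a save-game data container for video settings and player state.
; Paired setters and getters store console commands and selected enums for graphics, shadows, anti-aliasing, post-processing, view distance, textures and effects.
; Another pair stores player transform, health and current level.
; The command setter clears the graphics and post-processing commands to None instead of storing the passed values.
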(fn SettingAllCommand
  (params (Graphics%20Save%20Command :type String) (Shadows%20Save%20Command :type String) (Anti%20Save%20Command :type String) (POST-PROCESSINGSave%20Command :type String) (VIEW%20DISTANCE%20Save%20Command :type String) (TEXTURE%20QUALITY%20Save%20Command :type String) (EFFECTS%20Save%20Command :type String))
  (bind _output_get (Variables|Default|SetGraphics%20Save%20Command ""))
  (bind _output_get_2 (Variables|Default|SetShadows%20Save%20Command Shadows%20Save%20Command))
  (bind _output_get_3 (Variables|Default|SetAnti%20Save%20Command Anti%20Save%20Command))
  (bind _output_get_4 (Variables|Default|SetPOST-PROCESSINGSave%20Command ""))
  (bind _output_get_5 (Variables|Default|SetVIEW%20DISTANCE%20Save%20Command VIEW%20DISTANCE%20Save%20Command))
  (bind _output_get_6 (Variables|Default|SetTEXTURE%20QUALITY%20Save%20Command TEXTURE%20QUALITY%20Save%20Command))
  (bind _output_get_7 (Variables|Default|SetEFFECTS%20Save%20Command EFFECTS%20Save%20Command))
  (return _output_get _output_get_2 _output_get_3 _output_get_4 _output_get_5 _output_get_6 _output_get_7))

(fn SettingAllEnums
  (params (Graphics%20Target :type E_LowToHigh%20Enum :default "NewEnumerator0") (Shadows%20Target :type E_LowToHigh%20Enum :default "NewEnumerator0") (Anti%20Target :type E_LowToHigh%20Enum :default "NewEnumerator0") (POST-PROCESSING%20Target :type E_LowToHigh%20Enum :default "NewEnumerator0") (VIEW%20DISTANCE%20Target :type E_LowToHigh%20Enum :default "NewEnumerator0") (TEXTURE%20QUALITY%20Target :type E_LowToHigh%20Enum :default "NewEnumerator0") (EFFECTS%20Target :type E_LowToHigh%20Enum :default "NewEnumerator0"))
  (Variables|Default|SetGraphics%20Target Graphics%20Target)
  (Variables|Default|SetShadows%20Target Shadows%20Target)
  (Variables|Default|SetAnti%20Target Anti%20Target)
  (Variables|Default|SetPOST-PROCESSING%20Target POST-PROCESSING%20Target)
  (Variables|Default|SetVIEW%20DISTANCE%20Target VIEW%20DISTANCE%20Target)
  (Variables|Default|SetTEXTURE%20QUALITY%20Target TEXTURE%20QUALITY%20Target)
  (Variables|Default|SetEFFECTS%20Target EFFECTS%20Target))

(fn GettingAllCommand
  (return (Variables|Default|GetGraphics%20Save%20Command) (Variables|Default|GetShadows%20Save%20Command) (Variables|Default|GetAnti%20Save%20Command) (Variables|Default|GetPOST-PROCESSINGSave%20Command) (Variables|Default|GetVIEW%20DISTANCE%20Save%20Command) (Variables|Default|GetTEXTURE%20QUALITY%20Save%20Command) (Variables|Default|GetEFFECTS%20Save%20Command)))

(fn GettingAllEnums
  (return (Variables|Default|GetGraphics%20Target) (Variables|Default|GetShadows%20Target) (Variables|Default|GetAnti%20Target) (Variables|Default|GetPOST-PROCESSING%20Target) (Variables|Default|GetVIEW%20DISTANCE%20Target) (Variables|Default|GetTEXTURE%20QUALITY%20Target) (Variables|Default|GetEFFECTS%20Target)))

(fn SetPlayetState
  (params (layer%20Location%20And%20Rotations :type Transform) (Player%20Health :type Float%20%28double-precision%29) (Current%20Level :type Name))
  (Variables|Default|SetPlayer%20Location%20And%20Rotations layer%20Location%20And%20Rotations)
  (Variables|Default|SetPlayer%20Health Player%20Health)
  (Variables|Default|SetCurrent%20Level Current%20Level))

(fn GetPlayerState
  (return (Variables|Default|GetPlayer%20Location%20And%20Rotations) (Variables|Default|GetPlayer%20Health) (Variables|Default|GetCurrent%20Level)))