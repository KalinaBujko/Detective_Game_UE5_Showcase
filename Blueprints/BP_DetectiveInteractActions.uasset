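; Detective interaction action that handles a character interacting with a target, identified by a gameplay tag type.
; PerformInteraction stores both participants, signals interaction begin, calls the parent implementation, then switches on the tag with no connected branches.
; Disconnected logic would start the target's GraphNarrationTarget narration, restore the target's original yaw afterward and signal interaction end.
; As wired, this graph never calls interaction end itself.
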(event Custom|CustomEvent)

(event EventPerformInteraction
  (params (InteractingCharacter :type Actor%20Object%20Reference) (InteractionTarget :type Actor%20Object%20Reference) (InteractionType :type Gameplay%20Tag%20Structure))
  (Variables|Default|SetInteracting%20Character InteractingCharacter)
  (Variables|Default|SetInteraction%20Target InteractionTarget)
  (Default|CallOnInteractionBegin)
  (|CallParentFunction (Variables|Default|GetInteracting%20Character) (Variables|Default|GetInteraction%20Target) InteractionType)
  (|SwitchGameplayTag InteractionType))

(fn GetInitialRotations
  (params (CharB :type Actor%20Object%20Reference))
  (return (.yaw (Transformation|GetActorRotation CharB))))