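; First main-story GraphQuest, "Welcome in Manchester": leads the player from the station through Chambers' map shop to detective Ben Hilton's office.
; BeginQuest plays the intro movie, and RunQuestScriptDTO routes script IDs to handlers updating objectives, HUD hints, TalkToMe markers and game time.
; SetWorldState configures each level from objective outcomes, spawning NPCs and moving gates and level changers.
; Six office clues unlock Ben's greeting trigger; finding him completes the quest and adds Quest 2.
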(event Custom|Check_Painting
  (Class|QuestGraph|ReplaceObjectiveParameters "Check_Painting" "(TagName=\"GraphQuest.ObjectiveState\")" "(TagName=\"GraphQuest.ObjectiveState.Completed\")" false)
  (Class|QuestGraph|SetObjectiveOutcome "Check_Painting" "Success" false)
  (Class|BPIDetectiveGameInstance|SetHudPrimaryText(Message) (Game|GetGameInstance) (Utilities|String|Append "Poszukaj ciekawostek na temat detektywa w jego biurze - " (Utilities|String|ToString(Integer) (.znalezioneznajdzki (CallFunction|CzyWszystkieZnajdzkiPrzeklikane))) "/" "6"))
  (if (.bState (CallFunction|CzyWszystkieZnajdzkiPrzeklikane))
    (CallFunction|SpawnBenTrigger)))

(event Custom|Check_PoliceCode
  (Class|QuestGraph|ReplaceObjectiveParameters "Check_PoliceCode" "(TagName=\"GraphQuest.ObjectiveState\")" "(TagName=\"GraphQuest.ObjectiveState.Completed\")" false)
  (Class|QuestGraph|SetObjectiveOutcome "Check_PoliceCode" "Success" false)
  (Class|BPIDetectiveGameInstance|SetHudPrimaryText(Message) (Game|GetGameInstance) (Utilities|String|Append "Poszukaj ciekawostek na temat detektywa w jego biurze - " (Utilities|String|ToString(Integer) (.znalezioneznajdzki (CallFunction|CzyWszystkieZnajdzkiPrzeklikane))) "/" "6"))
  (if (.bState (CallFunction|CzyWszystkieZnajdzkiPrzeklikane))
    (CallFunction|SpawnBenTrigger)))

(event Custom|NewspaperMurdersInfo
  ;[0 0.000581 0.005] Gracz dostal gazete od chlopca i to jest drugie info o morderstwie
  (Class|QuestGraph|ReplaceObjectiveParameters "NewspaperMurdersInfo" "(TagName=\"GraphQuest.ObjectiveState\")" "(TagName=\"GraphQuest.ObjectiveState.Completed\")" false)
  (Class|QuestGraph|SetObjectiveOutcome "NewspaperMurdersInfo" "Success" false))

(event Custom|BenHiltonOfficeGreeing
  (bind _benhilton (CallFunction|BenEntersOffice))
  (Utilities|FlowControl|Delay 1.0)
  (Class|GraphNarrationTarget|BeginNarrationGraph (Actor|GetComponentbyClass _benhilton "/Script/SimpleNarration.GraphNarrationTarget") (Utilities|Array|MakeArray _benhilton) "/Game/_Main/Mechanics/Narration/Graphs/BP_BenHiltonOfficeGreeting.BP_BenHiltonOfficeGreeting_C"))

(event Custom|FindBenHilton
  (params (DTO :type Array%20of%20Object%20Object%20References))
  (bind _output (Utilities|Array|Get(acopy) DTO))
  (bind _asactor (Utilities|Casting|CastToActor _output))
  (Class|NarrationVariablesContainer|SetNarrationBool (Subsystems|GetNarrationVariablesContainer) _asactor "TalkToMePrimary" false)
  (Default|UpdateWidget (Actor|GetComponentbyClass _asactor "/Game/_Main/Mechanics/Narration/TalkToMe/BP_TalkToMe.BP_TalkToMe_C"))
  (Class|QuestGraph|SetObjectiveOutcome "FindBenHilton" "Success" false)
  (Class|QuestGraph|ReplaceObjectiveParameters "FindBenHilton" "(TagName=\"GraphQuest.ObjectiveState\")" "(TagName=\"GraphQuest.ObjectiveState.Completed\")" false)
  ;[0.3179 0.12 1] Cutscena nr 3
  ;
  ; Wyrzucenie z officu
  (Class|SMPStatics|PlayMovie "/SMP/BP_SMP_Player.BP_SMP_Player_C" "/Game/Movies/Cutscena_3_Compressed.Cutscena_3_Compressed" (Game|GetPlayerController 0) true 0.1 (Utilities|Set|MakeSet) (delegate Custom|CustomEvent_2))
  (CallFunction|SetGameTime 18))

(event Custom|Cawd
  (Class|QuestGraph|SetObjectiveOutcome "InitialCutscene" "Success" false)
  (Class|BPIDetectiveGameInstance|SetHudPrimaryText(Message) (Game|GetGameInstance) "Porozmawiaj z mieszkańcami - może ktoś będzie wiedział jak znaleźć detektywa Bena Hiltona")
  (Class|BPIDetectiveGameInstance|SetHudTip(Message) (Game|GetGameInstance))
  ;[0 0.000581 0.005] START GRY
  (Class|LevelChangeManager|OpenLevel(byName) (Subsystems|GetLevelChangeManager) "/Game/_Main/Levels/City/MainCity/BlockoutCityNat.BlockoutCityNat" true 1.0 "PlayerStartTag=1"))

(event Custom|CustomEvent
  (Class|QuestGraph|SetObjectiveOutcome "InitialCutscene" "Success" false)
  (Class|BPIDetectiveGameInstance|SetHudPrimaryText(Message) (Game|GetGameInstance) "Porozmawiaj z mieszkańcami - może ktoś będzie wiedział jak znaleźć detektywa Bena Hiltona")
  (Class|BPIDetectiveGameInstance|SetHudTip(Message) (Game|GetGameInstance)))

(event Custom|CustomEvent_2
  ;[0.3179 0.12 1] Cutscena nr 3
  ;
  ; Wyrzucenie z officu
  (Class|QuestGraph|ReplaceQuestParameters "(TagName=\"GraphQuest.QuestState\")" "(TagName=\"GraphQuest.QuestState.Completed\")" false)
  ;[1 0.5957 0] Add QUEST 2
  (Class|GraphQuestStatics|AddGraphQuest "WillsonHellberg" "BP_GraphQuest_Quest2" "/Game/_Main/Mechanics/Quests/BP_GraphQuest_Quest2.BP_GraphQuest_Quest2_C" (Utilities|Map|MakeMap) false)
  ;[0 0.000581 0.005] Wyjdz z office
  (bind _returnvalue (Actor|GetActorOfClass "/Game/_Main/Mechanics/LevelChangeSpot/BP_LevelChangeSpot.BP_LevelChangeSpot_C"))
  (Default|Interact _returnvalue)
  (CallFunction|SetGameTime 19))

(event Custom|CustomEvent_4
  ;[0.3179 0.12 1] Cutscenka: Rozmawiamy z sekretarką Bena, mamy zaczekać w gabinecie.”
  ;[0 0.000581 0.005] Make props  interactable
  (bind _outactors (Actor|GetAllActorsOfClass "/Game/_Main/Mechanics/Quests/QuestProps/BP_OfficeProp.BP_OfficeProp_C"))
  (for _array_element _outactors
    (Collision|SetCollisionEnabled (Variables|/Game/_Main/Mechanics/Quests/QuestProps/BP_OfficeProp.BP_OfficeProp_C|GetClickArea _array_element) "QueryOnly")
    (Class|BPIDetectiveGameInstance|SetHudPrimaryText(Message) (Game|GetGameInstance) "Poszukaj ciekawostek na temat detektywa w jego biurze")
    (Class|BPIDetectiveGameInstance|SetHudTip(Message) (Game|GetGameInstance))
    (Utilities|FlowControl|Delay 5.0)
    (Class|BPIDetectiveGameInstance|SetHudTip(Message) (Game|GetGameInstance) "Niektóre elementy odstają od reszty..."))
  (for _array_element_2 (Variables|Default|GetWszystkieZnajdzki)
    (Class|QuestGraph|ReplaceObjectiveParameters _array_element_2 "(TagName=\"GraphQuest.ObjectiveState\")" "(TagName=\"GraphQuest.ObjectiveState.InProgress\")" false)))

(event Custom|Check_Protocol
  (Class|QuestGraph|ReplaceObjectiveParameters "Check_Protocol" "(TagName=\"GraphQuest.ObjectiveState\")" "(TagName=\"GraphQuest.ObjectiveState.Completed\")" false)
  (Class|QuestGraph|SetObjectiveOutcome "Check_Protocol" "Success" false)
  (Class|BPIDetectiveGameInstance|SetHudPrimaryText(Message) (Game|GetGameInstance) (Utilities|String|Append "Poszukaj ciekawostek na temat detektywa w jego biurze - " (Utilities|String|ToString(Integer) (.znalezioneznajdzki (CallFunction|CzyWszystkieZnajdzkiPrzeklikane))) "/" "6"))
  (if (.bState (CallFunction|CzyWszystkieZnajdzkiPrzeklikane))
    (CallFunction|SpawnBenTrigger)))

(event Custom|Check_Knife
  (Class|QuestGraph|ReplaceObjectiveParameters "Check_Knife" "(TagName=\"GraphQuest.ObjectiveState\")" "(TagName=\"GraphQuest.ObjectiveState.Completed\")" false)
  (Class|QuestGraph|SetObjectiveOutcome "Check_Knife" "Success" false)
  (Class|BPIDetectiveGameInstance|SetHudPrimaryText(Message) (Game|GetGameInstance) (Utilities|String|Append "Poszukaj ciekawostek na temat detektywa w jego biurze - " (Utilities|String|ToString(Integer) (.znalezioneznajdzki (CallFunction|CzyWszystkieZnajdzkiPrzeklikane))) "/" "6"))
  (if (.bState (CallFunction|CzyWszystkieZnajdzkiPrzeklikane))
    (CallFunction|SpawnBenTrigger)))

(event Custom|Check_Raport
  (Class|QuestGraph|ReplaceObjectiveParameters "Check_Raport" "(TagName=\"GraphQuest.ObjectiveState\")" "(TagName=\"GraphQuest.ObjectiveState.Completed\")" false)
  (Class|QuestGraph|SetObjectiveOutcome "Check_Raport" "Success" false)
  (Class|BPIDetectiveGameInstance|SetHudPrimaryText(Message) (Game|GetGameInstance) (Utilities|String|Append "Poszukaj ciekawostek na temat detektywa w jego biurze - " (Utilities|String|ToString(Integer) (.znalezioneznajdzki (CallFunction|CzyWszystkieZnajdzkiPrzeklikane))) "/" "6"))
  (if (.bState (CallFunction|CzyWszystkieZnajdzkiPrzeklikane))
    (CallFunction|SpawnBenTrigger)))

(event Custom|Check_Tissue
  (Class|QuestGraph|ReplaceObjectiveParameters "Check_Tissue" "(TagName=\"GraphQuest.ObjectiveState\")" "(TagName=\"GraphQuest.ObjectiveState.Completed\")" false)
  (Class|QuestGraph|SetObjectiveOutcome "Check_Tissue" "Success" false)
  (Class|BPIDetectiveGameInstance|SetHudPrimaryText(Message) (Game|GetGameInstance) (Utilities|String|Append "Poszukaj ciekawostek na temat detektywa w jego biurze - " (Utilities|String|ToString(Integer) (.znalezioneznajdzki (CallFunction|CzyWszystkieZnajdzkiPrzeklikane))) "/" "6"))
  (if (.bState (CallFunction|CzyWszystkieZnajdzkiPrzeklikane))
    (CallFunction|SpawnBenTrigger)))

(event Custom|TalkToNewspaperBoy
  (params (DTO :type Array%20of%20Object%20Object%20References))
  (bind _output (Utilities|Array|Get(acopy) DTO))
  (bind _asactor (Utilities|Casting|CastToActor _output))
  (Class|QuestGraph|SetObjectiveOutcome "TalkToNewspaperBoy" "Success" false)
  (Class|QuestGraph|ReplaceObjectiveParameters "TalkToNewspaperBoy" "(TagName=\"GraphQuest.ObjectiveState\")" "(TagName=\"GraphQuest.ObjectiveState.Completed\")" false)
  (Utilities|FlowControl|Sequence
    (:then_0
      (Class|NarrationVariablesContainer|SetNarrationBool (Subsystems|GetNarrationVariablesContainer) _asactor "TalkToMePrimary" false)
      ;[0 0.000581 0.005] Bcs od Teraz Boy with newspapers moze dac side quest graczowi
      (Class|NarrationVariablesContainer|SetNarrationBool (Subsystems|GetNarrationVariablesContainer) _asactor "TalkToMeSecondary" true)
      (Default|UpdateWidget (Actor|GetComponentbyClass _asactor "/Game/_Main/Mechanics/Narration/TalkToMe/BP_TalkToMe.BP_TalkToMe_C")))
    (:then_1
      ;[0 0.000581 0.005] Platform npc tracą TalkToMe
      (bind _outactors (Actor|GetAllActorsOfClass "/Game/_Main/Mechanics/Characters/BP_PlatrormNPC0.BP_PlatrormNPC0_C"))
      (for _array_element _outactors
        (Class|NarrationVariablesContainer|SetNarrationBool (Subsystems|GetNarrationVariablesContainer) _array_element "TalkToMe" false)
        (Default|UpdateWidget (Actor|GetComponentbyClass _array_element "/Game/_Main/Mechanics/Narration/TalkToMe/BP_TalkToMe.BP_TalkToMe_C")))
      ;[1 1 1] Gracz dociera na rynek. Na rynku stoją npc, nie z każdym da się porozmawiać – możemy ich zapytać, gdzie znajduje się sklep lub poszukać go na własną rękę.
      ;;[0 0.000581 0.005] Na rynku wyspawnuj MarketNPC
      (CallFunction|SpawnMarketNPCs1))
    (:then_2
      (Class|BPIDetectiveGameInstance|SetHudPrimaryText(Message) (Game|GetGameInstance) "Znajdz sklep Pana Chambersa żeby zdobyć mape")
      (Class|BPIDetectiveGameInstance|SetHudTip(Message) (Game|GetGameInstance) "Sklep Pana Chambersa znajduje się niedaleko fontanny"))))

(event Custom|BuyMap
  (params (DTO :type Array%20of%20Object%20Object%20References))
  (bind _output (Utilities|Array|Get(acopy) DTO))
  (bind _asactor (Utilities|Casting|CastToActor _output))
  (CallFunction|SetGameTime 14)
  (Class|GraphQuestStatics|SetObjectiveOutcome "WillsonHellberg" "BP_GraphQuest_WelcomeInManchester" "BuyMap" "Success" false)
  (Class|GraphQuestStatics|ReplaceObjectiveParameters "WillsonHellberg" "BP_GraphQuest_WelcomeInManchester" "BuyMap" "(TagName=\"GraphQuest.ObjectiveState\")" "(TagName=\"GraphQuest.ObjectiveState.Completed\")" false)
  (Utilities|FlowControl|Sequence
    (:then_0
      ;[0 0.000581 0.005] Side quest
      (Utilities|FlowControl|Sequence
        (:then_0
          (Class|NarrationVariablesContainer|SetNarrationBool (Subsystems|GetNarrationVariablesContainer) _asactor "TalkToMePrimary" false)
          (bind _returnvalue (Class|GraphQuestStatics|HasGraphQuest "WillsonHellberg" "BP_GraphQUest_FetchNewspapers"))
          (if _returnvalue
            (Class|NarrationVariablesContainer|SetNarrationBool (Subsystems|GetNarrationVariablesContainer) _asactor "TalkToMeSecondary" true)))
        (:then_1
          (Default|UpdateWidget (Actor|GetComponentbyClass _asactor "/Game/_Main/Mechanics/Narration/TalkToMe/BP_TalkToMe.BP_TalkToMe_C")))))
    (:then_1
      (Class|QuestGraph|ReplaceObjectiveParameters "FindBenHilton" "(TagName=\"GraphQuest.ObjectiveState\")" "(TagName=\"GraphQuest.ObjectiveState.InProgress\")" false))
    (:then_2
      (Class|BPIDetectiveGameInstance|SetHudPrimaryText(Message) (Game|GetGameInstance) "Znajdz biuro Detektywa Bena")
      (Class|BPIDetectiveGameInstance|SetHudTip(Message) (Game|GetGameInstance) "Detektyw Ben to szanowany obywatel Manchesteru a budynek jego biura ma białą elewacje."))))

(event Custom|ChambersMurderInfoSuccess
  ;[0 0.000581 0.005] Gracz zapytal chambersa o morderstwo i otrzymap pierwsze info
  (Class|QuestGraph|ReplaceObjectiveParameters "ChambersMurderInfo" "(TagName=\"GraphQuest.ObjectiveState\")" "(TagName=\"GraphQuest.ObjectiveState.Completed\")" false)
  (Class|QuestGraph|SetObjectiveOutcome "ChambersMurderInfo" "Success" false))

(event Custom|ChambersMurderInfoFailure
  ;[0 0.000581 0.005] Gracz nie zapytal o morderstwo i szansa przepadla
  (Class|QuestGraph|ReplaceObjectiveParameters "ChambersMurderInfo" "(TagName=\"GraphQuest.ObjectiveState\")" "(TagName=\"GraphQuest.ObjectiveState.Failed\")" false)
  (Class|QuestGraph|SetObjectiveOutcome "ChambersMurderInfo" "Failure" false))

(event EventBeginQuest
  (Class|QuestGraph|ReplaceQuestParameters "(TagName=\"GraphQuest.QuestState\")" "(TagName=\"GraphQuest.QuestState.InProgress\")" false)
  (Class|QuestGraph|ReplaceObjectiveParameters "TalkToNewspaperBoy" "(TagName=\"GraphQuest.ObjectiveState\")" "(TagName=\"GraphQuest.ObjectiveState.InProgress\")" false)
  (Class|QuestGraph|ReplaceObjectiveParameters "BuyMap" "(TagName=\"GraphQuest.ObjectiveState\")" "(TagName=\"GraphQuest.ObjectiveState.InProgress\")" false)
  (Class|QuestGraph|ReplaceObjectiveParameters "ChambersMurderInfo" "(TagName=\"GraphQuest.ObjectiveState\")" "(TagName=\"GraphQuest.ObjectiveState.InProgress\")" false)
  (Class|QuestGraph|ReplaceObjectiveParameters "NewspaperMurdersInfo" "(TagName=\"GraphQuest.ObjectiveState\")" "(TagName=\"GraphQuest.ObjectiveState.InProgress\")" false)
  (Class|LowEntryExtendedStandardLibrary|DelayFrames)
  (Utilities|IsValid (Game|GetPlayerController 0)
    (:Is%20Valid
      _)
    (:Is%20Not%20Valid
      (Utilities|FlowControl|DelayUntilNextTick)))
  (bind _outcome (Class|QuestGraph|GetObjectiveOutcome "InitialCutscene"))
  (switch name _outcome
    (:None
      (Class|SMPStatics|PlayMovie "/SMP/BP_SMP_Player.BP_SMP_Player_C" "/Game/Movies/Cutscena_1_Compressed.Cutscena_1_Compressed" (Game|GetPlayerController 0) true 0.1 (Utilities|Set|MakeSet) (delegate Custom|Cawd))
      (CallFunction|SetGameTime 8))))

(event EventRunQuestScriptDTO
  (params (ScriptID :type Name :default "None") (DTO :type Array%20of%20Object%20Object%20References))
  (switch name ScriptID
    (:TalkToNewspaperBoy
      (CallFunction|TalktoNewspaperBoy DTO))
    (:BuyMap
      (CallFunction|BuyMap DTO))
    (:ChambersMurderInfoSuccess
      (CallFunction|ChambersMurderInfoSuccess))
    (:ChambersMurderInfoFailure
      (CallFunction|ChambersMurderInfoFailure))
    (:NewspaperMurdersInfo
      (CallFunction|NewspaperMurdersInfo))
    (:Check_Painting
      ;[0 0.000581 0.005] Biuro bena znajdzki
      (CallFunction|CheckPainting))
    (:Check_PoliceCode
      (CallFunction|CheckPoliceCode))
    (:Check_Protocol
      (CallFunction|CheckProtocol))
    (:Check_Knife
      (CallFunction|CheckKnife))
    (:Check_Raport
      (CallFunction|CheckRaport))
    (:Check_Tissue
      (CallFunction|CheckTissue))
    (:BenHiltonOfficeGreeting
      (CallFunction|BenHiltonOfficeGreeing))
    (:FindBenHilton
      (CallFunction|FindBenHilton DTO))))

(event EventSetWorldState
  (bind _returnvalue (Class|QuestGraph|CurrentWorldIs "/Game/_Main/Levels/City/MainCity/BlockoutCityNat.BlockoutCityNat"))
  (if _returnvalue
    (Utilities|FlowControl|Sequence
      (:then_1
        (bind _returnvalue_2 (Class|QuestGraph|GetObjectiveOutcome "BuyMap"))
        (if _returnvalue_2 ; False-> Nie udalo sie jeszcze wykonac tego objective
          (CallFunction|CloseParkGate)
          (else
            (CallFunction|CloseShopGates)))
        (bind _returnvalue_3 (Class|QuestGraph|GetObjectiveOutcome "TalkToNewspaperBoy"))
        (if (not _returnvalue_3) ; False-> Nie udalo sie jeszcze wykonac tego objective
          ;[1 1 1] Wyspawnuj npc na peronie
          (CallFunction|SpawnPlatformNPC)
          ;[0 0.000581 0.005] Show TalkToMe widget for BoyWithNewspapers
          (bind _returnvalue_4 (Actor|GetActorOfClass "/Game/_Main/Mechanics/Characters/BP_BoyWithNewspapers.BP_BoyWithNewspapers_C"))
          (Class|NarrationVariablesContainer|SetNarrationBool (Subsystems|GetNarrationVariablesContainer) _returnvalue_4 "TalkToMePrimary" true)
          (Default|UpdateWidget (Actor|GetComponentbyClass _returnvalue_4 "/Game/_Main/Mechanics/Narration/TalkToMe/BP_TalkToMe.BP_TalkToMe_C"))))
      (:then_2
        ;[0 0.000581 0.005] Otworz lub zamknij Wejscie do Bena
        (bind _outcome (Class|QuestGraph|GetObjectiveOutcome "FindBenHilton"))
        (switch name _outcome
          (:Success
            ;[0 0.000581 0.005] Zamknij
            (bind _outactors (Actor|GetAllActorswithTag "LevelChangerOffice"))
            (Transformation|SetActorLocation (Utilities|Array|Get(acopy) _outactors) (+ (Transformation|GetActorLocation (Utilities|Array|Get(acopy) _outactors)) "0.000000,0.000000,1000.000000") false false))))
      (:then_3
        ;[1 1 1] Nie mozemy jeszcze wejsc do burdello
        (bind _outcome_2 (Class|QuestGraph|GetObjectiveOutcome "FindBenHilton"))
        (switch name _outcome_2
          (:None
            (bind _outactors_2 (Actor|GetAllActorswithTag "LevelChangerBurdel"))
            (Transformation|SetActorLocation (Utilities|Array|Get(acopy) _outactors_2) (+ (Transformation|GetActorLocation (Utilities|Array|Get(acopy) _outactors_2)) "0.000000,0.000000,2000.000000") false false)))))
    (else
      (bind _returnvalue_5 (Class|QuestGraph|CurrentWorldIs "/Game/_Main/Levels/ClosedLocations/Shop.Shop"))
      (if _returnvalue_5
        (bind _outcome_3 (Class|QuestGraph|GetObjectiveOutcome "BuyMap"))
        (switch name _outcome_3
          (:None
            (bind _outactors_3 (Actor|GetAllActorswithInterface "/Game/_Main/Mechanics/Characters/BPI_Chambers.BPI_Chambers_C"))
            (Class|NarrationVariablesContainer|SetNarrationBool (Subsystems|GetNarrationVariablesContainer) (Utilities|Array|Get(acopy) _outactors_3) "TalkToMePrimary" true)
            (Default|UpdateWidget (Actor|GetComponentbyClass (Utilities|Array|Get(acopy) _outactors_3) "/Game/_Main/Mechanics/Narration/TalkToMe/BP_TalkToMe.BP_TalkToMe_C"))))
        (else
          ;[0 0.000581 0.005] Gdy jestesmy w biurze bena
          (bind _returnvalue_6 (Class|QuestGraph|CurrentWorldIs "/Game/_Main/Levels/ClosedLocations/Office.Office"))
          (if _returnvalue_6
            (bind _outcome_4 (Class|QuestGraph|GetObjectiveOutcome "FindBenHilton"))
            (switch name _outcome_4
              (:None
                ;[0 0.000581 0.005] Wylacz drzwi wyjsciiowe
                (bind _returnvalue_7 (Actor|GetActorOfClass "/Game/_Main/Mechanics/LevelChangeSpot/BP_LevelChangeSpot.BP_LevelChangeSpot_C"))
                (Transformation|SetActorLocation _returnvalue_7 (+ (Transformation|GetActorLocation _returnvalue_7) "0.000000,0.000000,1000.000000") false false)
                (Class|LowEntryExtendedStandardLibrary|DelayFrames)
                ;[0.3179 0.12 1] Cutscenka: Rozmawiamy z sekretarką Bena, mamy zaczekać w gabinecie.”
                (Utilities|IsValid (Game|GetPlayerController 0)
                  (:Is%20Valid
                    _)
                  (:Is%20Not%20Valid
                    (Utilities|FlowControl|DelayUntilNextTick)))
                (Class|SMPStatics|PlayMovie "/SMP/BP_SMP_Player.BP_SMP_Player_C" "/Game/Movies/Cutscena_2_Compressed.Cutscena_2_Compressed" (Game|GetPlayerController 0) true 0.1 (Utilities|Set|MakeSet) (delegate Custom|CustomEvent_4))))))))))

(fn GetDefaultQuestData
  (return (Utilities|Struct|MakeGraphQuestData (Utilities|Map|MakeMap "(TagName=\"GraphQuest.QuestText.Title\")" "QUEST 1" "(TagName=\"GraphQuest.QuestText.Description\")" "- Znajdź detektywa Bena. 
- Znajdź sklep i kup mapę miasta. 
- Dowiedz się czegoś o morderstwach.") "(GameplayTags=)" (Class|QuestGraph|AppendObjectives (Utilities|Map|MakeMap "InitialCutscene" (Utilities|Struct|MakeGraphQuestObjective (Utilities|Map|MakeMap "(TagName=\"GraphQuest.ObjectiveText.Title\")" "Initial Cutscene" "(TagName=\"GraphQuest.ObjectiveText.Description\")" "Initial Cutscene") "(GameplayTags=((TagName=\"GraphQuest.ObjectiveParameter.Hidden\")))")) (Class|QuestGraph|AppendObjectives (Utilities|Map|MakeMap "TalkToNewspaperBoy" (Utilities|Struct|MakeGraphQuestObjective (Utilities|Map|MakeMap "(TagName=\"GraphQuest.ObjectiveText.Title\")" "Gdzie znajdę tego chuja Bena" "(TagName=\"GraphQuest.ObjectiveText.Description\")" "Rozejrzyj się po okolicach dworca może dowiesz sie czegos o morderstwach lub przynajmniej gdzie można znalezc Bena.") "(GameplayTags=)") "BuyMap" (Utilities|Struct|MakeGraphQuestObjective (Utilities|Map|MakeMap "(TagName=\"GraphQuest.ObjectiveText.Title\")" "Kup mapę miasta." "(TagName=\"GraphQuest.ObjectiveText.Description\")" "Znajdź sklep i kup mapę miasta.") "(GameplayTags=)") "ChambersMurderInfo" (Utilities|Struct|MakeGraphQuestObjective (Utilities|Map|MakeMap "(TagName=\"GraphQuest.ObjectiveText.Title\")" "Dowiedz się czegoś o morderstwach" "(TagName=\"GraphQuest.ObjectiveText.Description\")" "Moze w jakims klepie ktos cos bedzie wiedzial ") "(GameplayTags=((TagName=\"GraphQuest.ObjectiveType.Optional\")))") "NewspaperMurdersInfo" (Utilities|Struct|MakeGraphQuestObjective (Utilities|Map|MakeMap "(TagName=\"GraphQuest.ObjectiveText.Title\")" "Dowiedz się czegoś o morderstwach" "(TagName=\"GraphQuest.ObjectiveText.Description\")" " ") "(GameplayTags=((TagName=\"GraphQuest.ObjectiveType.Optional\")))")) (Utilities|Map|MakeMap "FindBenHilton" (Utilities|Struct|MakeGraphQuestObjective (Utilities|Map|MakeMap "(TagName=\"GraphQuest.ObjectiveText.Title\")" "Znajdz detektywa Bena Hiltona" "(TagName=\"GraphQuest.ObjectiveText.Description\")" "Znajdz tego chuja bena") "(GameplayTags=)") "Check_Painting" (Utilities|Struct|MakeGraphQuestObjective (Utilities|Map|MakeMap "(TagName=\"GraphQuest.ObjectiveText.Title\")" "Portret na scianie" "(TagName=\"GraphQuest.ObjectiveText.Description\")" "Na ścianie wisi Portret Bena i Franka – na dole portretu jest dopisek kogo on przedstawia") "(GameplayTags=)") "Check_PoliceCode" (Utilities|Struct|MakeGraphQuestObjective (Utilities|Map|MakeMap "(TagName=\"GraphQuest.ObjectiveText.Title\")" "Stół" "(TagName=\"GraphQuest.ObjectiveText.Description\")" "Na Stole leży Kodeks Policyjny") "(GameplayTags=)") "Check_Protocol" (Utilities|Struct|MakeGraphQuestObjective (Utilities|Map|MakeMap "(TagName=\"GraphQuest.ObjectiveText.Title\")" "Biurko" "(TagName=\"GraphQuest.ObjectiveText.Description\")" "Na biurku leży protokół z przesłuchania sprawcy") "(GameplayTags=)") "Check_Knife" (Utilities|Struct|MakeGraphQuestObjective (Utilities|Map|MakeMap "(TagName=\"GraphQuest.ObjectiveText.Title\")" "Knife" "(TagName=\"GraphQuest.ObjectiveText.Description\")" "Na półce/szafce leży Nóż Absolwenta.") "(GameplayTags=)") "Check_Raport" (Utilities|Struct|MakeGraphQuestObjective (Utilities|Map|MakeMap "(TagName=\"GraphQuest.ObjectiveText.Title\")" "Knife" "(TagName=\"GraphQuest.ObjectiveText.Description\")" "Na półce/szafce leży Nóż Absolwenta.") "(GameplayTags=)") "Check_Tissue" (Utilities|Struct|MakeGraphQuestObjective (Utilities|Map|MakeMap "(TagName=\"GraphQuest.ObjectiveText.Title\")" "Tissue" "(TagName=\"GraphQuest.ObjectiveText.Description\")" "Chusteczka z Czterołapego Łabędzia") "(GameplayTags=)")))))))

(fn SpawnMarketNPCs1
  (for _array_element (LocalVariables|GetMarketNPCs)
    ;[0 0.000581 0.005] Wyspawnuj BP_PlatrormNPCs
    (bind _returnvalue (Game|SpawnActorfromClass "/Game/_Main/Mechanics/Characters/BP_MarketNPC1.BP_MarketNPC1_C" _array_element "AlwaysSpawn" "MultiplyWithRoot" 0 0))
    ;[0 0.000581 0.005] Show TalkToMe widget for PlatformNPC
    (Class|NarrationVariablesContainer|SetNarrationBool (Subsystems|GetNarrationVariablesContainer) _returnvalue "TalkToMe" true)
    (Default|UpdateWidget (Utilities|Array|Get(acopy) (Actor|GetComponentsByClass _returnvalue "/Game/_Main/Mechanics/Narration/TalkToMe/BP_TalkToMe.BP_TalkToMe_C")))))

(fn CloseShopGates
  (bind _outactors (Actor|GetAllActorsOfClasswithTag "/Game/_Main/Art/Props/Wall/BP_Gate.BP_Gate_C" "GateShop0"))
  (Default|SetOpen (Utilities|Array|Get(acopy) _outactors) false)
  (bind _outactors_2 (Actor|GetAllActorsOfClasswithTag "/Game/_Main/Art/Props/Wall/BP_Gate.BP_Gate_C" "GateShop1"))
  (Default|SetOpen (Utilities|Array|Get(acopy) _outactors_2) false))

(fn CloseParkGate
  (bind _outactors (Actor|GetAllActorsOfClasswithTag "/Game/_Main/Art/Props/Wall/BP_Gate.BP_Gate_C" "GatePark0"))
  (Default|SetOpen (Utilities|Array|Get(acopy) _outactors) false))

(fn CzyWszystkieZnajdzkiPrzeklikane
  (bind _znajdzki (LocalVariables|GetZnajdzki))
  (for _array_element (Variables|Default|GetWszystkieZnajdzki)
    (bind _outcome (Class|QuestGraph|GetObjectiveOutcome _array_element))
    (switch name _outcome
      (:Success
        (Math|Integer|IncrementInt (LocalVariables|GetZnajdzki)))))
  (return (>= _znajdzki 6) _znajdzki))

(fn BenEntersOffice
  (bind _returnvalue (Game|SpawnActorfromClass "/Game/_Main/Mechanics/Characters/BP_BenHilton.BP_BenHilton_C" (Math|Transform|MakeTransform "0.000000,-310.000000,91.000000" "0.000000,60.000000,0.000000" "1.000000,1.000000,1.000000") "AlwaysSpawn" "MultiplyWithRoot" 0 0))
  (Class|NarrationVariablesContainer|SetNarrationBool (Subsystems|GetNarrationVariablesContainer) _returnvalue "TalkToMePrimary" true)
  (Default|UpdateWidget (Actor|GetComponentbyClass _returnvalue "/Game/_Main/Mechanics/Narration/TalkToMe/BP_TalkToMe.BP_TalkToMe_C"))
  (return _returnvalue))

(fn SpawnBenTrigger
  (bind _returnvalue (Game|SpawnActorfromClass "/Game/_Main/Mechanics/Quests/QuestProps/BP_GraphQuest_RunScriptTrigger.BP_GraphQuest_RunScriptTrigger_C" (Math|Transform|MakeTransform "260.000000,30.000000,70.000000" "0, 0, 0" "2.500000,1.000000,2.000000") "AlwaysSpawn" "MultiplyWithRoot" 0 0))
  (Variables|/Game/_Main/Mechanics/Quests/QuestProps/BP_GraphQuest_RunScriptTrigger.BP_GraphQuest_RunScriptTrigger_C|SetCharacterID _returnvalue "WillsonHellberg")
  (Variables|/Game/_Main/Mechanics/Quests/QuestProps/BP_GraphQuest_RunScriptTrigger.BP_GraphQuest_RunScriptTrigger_C|SetQuest%20ID _returnvalue "BP_GraphQuest_WelcomeInManchester")
  (Variables|/Game/_Main/Mechanics/Quests/QuestProps/BP_GraphQuest_RunScriptTrigger.BP_GraphQuest_RunScriptTrigger_C|SetScriptID _returnvalue "BenHiltonOfficeGreeting"))

(fn SpawnPlatformNPC
  (for _array_element (LocalVariables|GetPlatformNPCs)
    ;[0 0.000581 0.005] Wyspawnuj BP_PlatrormNPCs
    (bind _returnvalue (Game|SpawnActorfromClass "/Game/_Main/Mechanics/Characters/BP_PlatrormNPC0.BP_PlatrormNPC0_C" _array_element "AlwaysSpawn" "MultiplyWithRoot" 0 0))
    ;[0 0.000581 0.005] Show TalkToMe widget for PlatformNPC
    (Class|NarrationVariablesContainer|SetNarrationBool (Subsystems|GetNarrationVariablesContainer) _returnvalue "TalkToMe" true)
    (Default|UpdateWidget (Utilities|Array|Get(acopy) (Actor|GetComponentsByClass _returnvalue "/Game/_Main/Mechanics/Narration/TalkToMe/BP_TalkToMe.BP_TalkToMe_C")))))