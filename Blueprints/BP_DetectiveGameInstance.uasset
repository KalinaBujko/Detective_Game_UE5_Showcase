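; Game instance for a detective game that sets up its plugins and holds shared HUD message state.
; On start it initializes game settings with example defaults, the level changer's transition widget, graph narration with detective widgets and custom actions, and click-to-interact.
; It stores the HUD reference, primary text and tip, and either text setter refreshes the HUD message.
; RemoveWidget only checks validity, as its RemoveFromParent call is disconnected.
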(event EventStart
  (CallFunction|InitGameSettings)
  (CallFunction|InitLevelChanger)
  (CallFunction|InitNarrationPlugin)
  (CallFunction|InitClickInteract))

(event EventSetHudPrimaryText
  (params (SetPrimaryText :type String))
  (Variables|Default|SetHUDPrimaryText SetPrimaryText)
  (Class|BPIHUD|UpdateHUD(Message) (stale EventSetHUD _output_get)))

(event EventSetHudTip
  (params (SetTipText :type String))
  (Variables|Default|SetHUDTip SetTipText)
  (Class|BPIHUD|UpdateHUD(Message) (stale EventSetHUD _output_get)))

(event EventSetHUD
  (params (Widget :type Widget%20Object%20Reference))
  (bind _output_get (Variables|Default|SetHUD Widget)))

(fn InitGameSettings
  (bind (_bool _int _float _input) (CallFunction|GetExampleDefaultSettings))
  (Class|GameSettingsController|InitializePlugin (Subsystems|GetGameSettingsController) "/GameSettings/SettingsControllers/BP_GraphicsSettingsController.BP_GraphicsSettingsController_C" 0 0 "/GameSettings/SettingsControllers/BP_InputSettingsController.BP_InputSettingsController_C" (CallFunction|GetExampleJsonSerializedSettings) (Class|BlueprintPathsLibrary|ProjectSavedDir) (Utilities|Set|MakeSet))
  (bind _returnvalue (Class|GameSettingsController|InitializeSettings (Subsystems|GetGameSettingsController) _bool _int _float _input))
  (if _returnvalue
    _))

(fn InitLevelChanger
  (Class|LevelChangeManager|InitializePlugin (Subsystems|GetLevelChangeManager) "/Game/_Main/UI/TransitionWIdget/WBP_Transition.WBP_Transition_C"))

(fn InitNarrationPlugin
  (Class|GraphNarrationController|InitializePlugin (Subsystems|GetGraphNarrationController) "/Game/_Main/Mechanics/Narration/System/WBP_Detective_ScreenNarrationWidget.WBP_Detective_ScreenNarrationWidget_C" "/Game/_Main/Mechanics/Narration/System/BP_Detective_NarrationCustomActions.BP_Detective_NarrationCustomActions_C" "/Game/_Main/Mechanics/Narration/System/WBP_Detective_SceneNarrationWidget.WBP_Detective_SceneNarrationWidget_C"))

(fn InitClickInteract
  (Class|ClickInteractController|InitializePlugin (Subsystems|GetClickInteractController) "(TagName=\"SceneComponent.ClickInteract.RangeArea\")" "(TagName=\"Actor.Character.Player\")"))

(fn RemoveWidget
  (params (WidgetToRemove :type Widget%20Object%20Reference))
  (Utilities|IsValid WidgetToRemove))

(fn GetHudPrimaryText
  (return (Variables|Default|GetHUDPrimaryText)))

(fn GetHudTip
  (return (Variables|Default|GetHUDTip)))