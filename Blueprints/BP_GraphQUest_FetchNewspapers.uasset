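; Two-objective fetch quest in which the player collects newspapers from Mr. Chambers and delivers them to a newspaper boy.
; Script IDs advance objective states and clear the TalkToMeSecondary narration flag on the actor passed via DTO, refreshing its TalkToMe widget.
; Delivery completes the quest and fires the murder-news script in WelcomeInManchester.
; SetWorldState re-flags the boy, found by interface, while delivery is pending.
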(event EventBeginQuest
  (Class|QuestGraph|ReplaceQuestParameters "(TagName=\"GraphQuest.QuestState\")" "(TagName=\"GraphQuest.QuestState.InProgress\")" false)
  (Class|QuestGraph|ReplaceObjectiveParameters "GetNewspapers" "(TagName=\"GraphQuest.ObjectiveState\")" "(TagName=\"GraphQuest.ObjectiveState.InProgress\")" false))

(event EventRunQuestScriptDTO
  (params (ScriptID :type Name :default "None") (DTO :type Array%20of%20Object%20Object%20References))
  (bind _output (Utilities|Array|Get(acopy) DTO))
  (bind _asactor (Utilities|Casting|CastToActor _output))
  (bind _asactor_2 (Utilities|Casting|CastToActor _output))
  (switch name ScriptID
    (:GetNewspapers
      ;[0 0.000581 0.005] Gracz wzial gazetuy od sprzedawcy
      (Class|QuestGraph|SetObjectiveOutcome "GetNewspapers" "Success" false)
      (Class|QuestGraph|ReplaceObjectiveParameters "GetNewspapers" "(TagName=\"GraphQuest.ObjectiveState\")" "(TagName=\"GraphQuest.ObjectiveState.Completed\")" false)
      (Class|QuestGraph|ReplaceObjectiveParameters "DeliverNewspapers" "(TagName=\"GraphQuest.ObjectiveState\")" "(TagName=\"GraphQuest.ObjectiveState.InProgress\")" false)
      (Class|NarrationVariablesContainer|SetNarrationBool (Subsystems|GetNarrationVariablesContainer) _asactor_2 "TalkToMeSecondary" false)
      (Default|UpdateWidget (Actor|GetComponentbyClass _asactor_2 "/Game/_Main/Mechanics/Narration/TalkToMe/BP_TalkToMe.BP_TalkToMe_C")))
    (:OnDeliverNewspapers
      (Class|QuestGraph|SetObjectiveOutcome "DeliverNewspapers" "Success" false)
      (Class|QuestGraph|ReplaceObjectiveParameters "DeliverNewspapers" "(TagName=\"GraphQuest.ObjectiveState\")" "(TagName=\"GraphQuest.ObjectiveState.Completed\")" false)
      (Class|NarrationVariablesContainer|SetNarrationBool (Subsystems|GetNarrationVariablesContainer) _asactor "TalkToMeSecondary" false)
      (Default|UpdateWidget (Actor|GetComponentbyClass _asactor "/Game/_Main/Mechanics/Narration/TalkToMe/BP_TalkToMe.BP_TalkToMe_C"))
      (Class|QuestGraph|ReplaceQuestParameters "(TagName=\"GraphQuest.QuestState\")" "(TagName=\"GraphQuest.QuestState.Completed\")" false)
      ;[0 0.000581 0.005] Bo w gazecie jest info o morderstwie
      (Class|GraphQuestStatics|RunQuestScript "WillsonHellberg" "BP_GraphQuest_WelcomeInManchester" "NewspaperMurdersInfo"))))

(event EventSetWorldState
  (Class|QuestGraph|CurrentWorldIs "/Game/_Main/Levels/City/MainCity/BlockoutCityNat.BlockoutCityNat")
  (bind _outcome (Class|QuestGraph|GetObjectiveOutcome "GetNewspapers"))
  (switch name _outcome
    (:Success
      (bind _outcome_2 (Class|QuestGraph|GetObjectiveOutcome "DeliverNewspapers"))
      (switch name _outcome_2
        (:None
          (bind _outactors (Actor|GetAllActorswithInterface "/Game/_Main/Mechanics/Characters/BPI_BoyWithNewspapers.BPI_BoyWithNewspapers_C"))
          (Class|NarrationVariablesContainer|SetNarrationBool (Subsystems|GetNarrationVariablesContainer) (Utilities|Array|Get(acopy) _outactors) "TalkToMeSecondary" true)
          (Default|UpdateWidget (Actor|GetComponentbyClass (Utilities|Array|Get(acopy) _outactors) "/Game/_Main/Mechanics/Narration/TalkToMe/BP_TalkToMe.BP_TalkToMe_C")))))))

(fn GetDefaultQuestData
  (return (Utilities|Struct|MakeGraphQuestData (Utilities|Map|MakeMap "(TagName=\"GraphQuest.QuestText.Title\")" "Fetch Newspapers" "(TagName=\"GraphQuest.QuestText.Description\")" "- Chlopiec z gazetami poprosil o dostarczenie mu nową partię.") "(GameplayTags=)" (Utilities|Map|MakeMap "GetNewspapers" (Utilities|Struct|MakeGraphQuestObjective (Utilities|Map|MakeMap "(TagName=\"GraphQuest.ObjectiveText.Title\")" "Wez gazety od pana Chambersa " "(TagName=\"GraphQuest.ObjectiveText.Description\")" "bla bla bal") "(GameplayTags=)") "DeliverNewspapers" (Utilities|Struct|MakeGraphQuestObjective (Utilities|Map|MakeMap "(TagName=\"GraphQuest.ObjectiveText.Title\")" "Dostarcz gazety chłopcu" "(TagName=\"GraphQuest.ObjectiveText.Description\")" "bla bla bal") "(GameplayTags=)")))))