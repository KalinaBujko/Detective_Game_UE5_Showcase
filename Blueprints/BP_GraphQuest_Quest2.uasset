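; GraphQuest asset for Quest 2, where Willson seeks a bed for the night in Manchester.
; SetWorldState stages each level: gates, officers, leaflets, beggars and hidden brothel entrance in the city, locked exit and barman talk inside.
; RunQuestScriptDTO dispatches script IDs that update objectives, HUD hints and TalkToMe prompts, leading from beggars through barman to Ann.
; Ann's first dialogue enables the bed, which plays a cutscene and then quits the game.
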(event Custom|AnnDialogue0
  (bind _returnvalue (Game|GetPlayerController 0))
  (bind _returnvalue_2 (Game|GetPlayerController 0))
  ;[0 0.000581 0.005] Willson porozmawial z Anka poraz pierwszy
  (Class|QuestGraph|SetObjectiveOutcome "AnnDialogue0" "Success" false)
  (Class|QuestGraph|ReplaceObjectiveParameters "AnnDialogue0" "(TagName=\"GraphQuest.ObjectiveState\")" "(TagName=\"GraphQuest.ObjectiveState.Completed\")" false)
  (Input|DisableInput (Pawn|GetControlledPawn _returnvalue_2) _returnvalue_2)
  ;[0 0.000581 0.005] Kurwa zfriendzonowala wilsona
  ; i wychodzi z pokoju zniesmaczona
  (bind _outactors (Actor|GetAllActorswithInterface "/Game/_Main/Mechanics/Characters/BPI_Ann.BPI_Ann_C"))
  (AI|AIMoveTo (Utilities|Array|Get(acopy) _outactors) (.AsPawn (Utilities|Casting|CastToPawn (Utilities|Array|Get(acopy) _outactors))) "495.542842,6386.666273,380.000000" 0 5.0 false
    (:then
      (Class|NarrationVariablesContainer|SetNarrationBool (Subsystems|GetNarrationVariablesContainer) (Utilities|Array|Get(acopy) _outactors) "TalkToMePrimary" false)
      (Class|NarrationVariablesContainer|SetNarrationBool (Subsystems|GetNarrationVariablesContainer) (Utilities|Array|Get(acopy) _outactors) "TalkToMeSecondary" true)
      (Default|UpdateWidget (Actor|GetComponentbyClass (Utilities|Array|Get(acopy) _outactors) "/Game/_Main/Mechanics/Narration/TalkToMe/BP_TalkToMe.BP_TalkToMe_C"))
      (Utilities|FlowControl|Delay 3.0)
      (Variables|/Script/Engine.CharacterMovementComponent|SetMaxWalkSpeed (Actor|GetComponentbyClass (Utilities|Array|Get(acopy) _outactors) "/Script/Engine.CharacterMovementComponent") 4.5e+02)
      (Utilities|FlowControl|Delay 1.0)
      (Input|EnableInput (Pawn|GetControlledPawn _returnvalue) _returnvalue))
    (:OnSuccess
      (Transformation|SetActorRotation (Utilities|Array|Get(acopy) _outactors) "0.000000,160.000000,0.000000" :!label _label)
      (bind _returnvalue_3 (Actor|GetActorOfClass "/Game/_Main/Mechanics/Quests/QuestProps/BP_Bed.BP_Bed_C"))
      (Collision|SetCollisionEnabled (Variables|/Game/_Main/Mechanics/Quests/QuestProps/BP_Bed.BP_Bed_C|GetClickArea _returnvalue_3) "QueryOnly")
      (Class|BPIDetectiveGameInstance|SetHudPrimaryText(Message) (Game|GetGameInstance) "Pójdź spać w pokoju nr 2")
      (Class|BPIDetectiveGameInstance|SetHudTip(Message) (Game|GetGameInstance) "Chyba Ania ma Ci coś jeszcze do powiedzenia..."))
    (:OnFail
      (Transformation|SetActorLocation (Utilities|Array|Get(acopy) _outactors) "495.542842,6386.666273,380.000000" false false)
      (goto _label))))

(event Custom|AnnDialogue1
  (Class|QuestGraph|SetObjectiveOutcome "AnnDialogue1" "Success" false)
  (Class|QuestGraph|ReplaceObjectiveParameters "AnnDialogue1" "(TagName=\"GraphQuest.ObjectiveState\")" "(TagName=\"GraphQuest.ObjectiveState.Completed\")" false)
  (bind _outactors (Actor|GetAllActorswithInterface "/Game/_Main/Mechanics/Characters/BPI_Ann.BPI_Ann_C"))
  (Class|NarrationVariablesContainer|SetNarrationBool (Subsystems|GetNarrationVariablesContainer) (Utilities|Array|Get(acopy) _outactors) "TalkToMeSecondary" false)
  (Default|UpdateWidget (Actor|GetComponentbyClass (Utilities|Array|Get(acopy) _outactors) "/Game/_Main/Mechanics/Narration/TalkToMe/BP_TalkToMe.BP_TalkToMe_C"))
  (Class|BPIDetectiveGameInstance|SetHudPrimaryText(Message) (Game|GetGameInstance) "Pójdź spać w pokoju nr 2")
  (Class|BPIDetectiveGameInstance|SetHudTip(Message) (Game|GetGameInstance)))

(event Custom|BedInteractedWith
  (bind _returnvalue (Game|GetPlayerController 0))
  ;[0 0.000581 0.005] PLay cutscenke
  (Input|DisableInput (Pawn|GetControlledPawn _returnvalue) _returnvalue)
  (Class|SMPStatics|PlayMovie "/SMP/BP_SMP_Player.BP_SMP_Player_C" "/Game/Movies/Cutscena_4_d.Cutscena_4_d" _returnvalue true 0.2 (Utilities|Set|MakeSet) (delegate Custom|CustomEvent_0)))

(event Custom|CustomEvent_0
  (Game|QuitGame 0 "Quit" false))

(event EventBeginQuest
  (Class|QuestGraph|ReplaceQuestParameters "(TagName=\"GraphQuest.QuestState\")" "(TagName=\"GraphQuest.QuestState.InProgress\")" false)
  (Class|QuestGraph|ReplaceObjectiveParameters "FindSleepingPlace" "(TagName=\"GraphQuest.ObjectiveState\")" "(TagName=\"GraphQuest.ObjectiveState.InProgress\")" false)
  (Class|QuestGraph|ReplaceObjectiveParameters "CoinFound" "(TagName=\"GraphQuest.ObjectiveState\")" "(TagName=\"GraphQuest.ObjectiveState.InProgress\")" false)
  (bind _returnvalue (Actor|GetActorOfClass "/Game/_Main/Mechanics/Characters/BP_WillsonHellberg.BP_WillsonHellberg_C"))
  (Class|QuestGraph|RunQuestScriptDTO "InitialCheckCoins" (Utilities|Array|MakeArray _returnvalue))
  (Class|BPIDetectiveGameInstance|SetHudPrimaryText(Message) (Game|GetGameInstance) "Spędź noc w Manchesterze")
  (Class|BPIDetectiveGameInstance|SetHudTip(Message) (Game|GetGameInstance) "Rozejrzyj się po mieście lub porozmawiaj z mieszkańcami żeby wynająć jakiś pokój lub łóźko. "))

(event EventRunQuestScriptDTO
  (params (ScriptID :type Name :default "None") (DTO :type Array%20of%20Object%20Object%20References))
  (bind _output (Utilities|Array|Get(acopy) DTO))
  (bind _output_2 (Utilities|Array|Get(acopy) DTO))
  (bind _asactor (Utilities|Casting|CastToActor _output_2))
  (bind _asactor_2 (Utilities|Casting|CastToActor _output))
  (switch name ScriptID
    (:BeggarTalkedTo
      (Class|NarrationVariablesContainer|SetNarrationBool (Subsystems|GetNarrationVariablesContainer) _asactor_2 "TalkToMePrimary" false)
      (Default|UpdateWidget (Actor|GetComponentbyClass _asactor_2 "/Game/_Main/Mechanics/Narration/TalkToMe/BP_TalkToMe.BP_TalkToMe_C"))
      (Class|QuestGraph|SetObjectiveOutcome "FindHostelsInfo" "Success" false)
      ;[0 0.000581 0.005] Odblokuj drzwi do burdelu
      (bind _outactors (Actor|GetAllActorsOfClasswithTag "/Game/_Main/Mechanics/LevelChangeSpot/BP_LevelChangeSpot.BP_LevelChangeSpot_C" "LevelChangerBurdel"))
      (Transformation|SetActorLocation (Utilities|Array|Get(acopy) _outactors) "12808.259539,31477.219894,253.828421" false false)
      (Class|BPIDetectiveGameInstance|SetHudPrimaryText(Message) (Game|GetGameInstance) "Udaj się do burdelu żeby wynająć pokój na noc.")
      (Class|BPIDetectiveGameInstance|SetHudTip(Message) (Game|GetGameInstance) "Burdel znajduję się w biednej dzielnicy zwanej \"Slumsami\""))
    (:CoinFound
      (Class|QuestGraph|SetObjectiveOutcome "CoinFound" "Success" false :!label _label))
    (:InitialCheckCoins
      (bind (_bsuccess _value) (Class|NarrationVariablesContainer|GetNarrationInt (Subsystems|GetNarrationVariablesContainer) (.AsActor (Utilities|Casting|CastToActor (Utilities|Array|Get(acopy) DTO))) "CoinsFound"))
      (if _bsuccess
        (if (> _value 0)
          (goto _label))))
    (:FindSleepingPlace
      ;[0 0.000581 0.005] Rozmowa z barmanem dobiegla konca
      (Class|QuestGraph|SetObjectiveOutcome "FindSleepingPlace" "Success" false)
      (Class|QuestGraph|ReplaceObjectiveParameters "FindSleepingPlace" "(TagName=\"GraphQuest.ObjectiveState\")" "(TagName=\"GraphQuest.ObjectiveState.Completed\")" false)
      (Class|NarrationVariablesContainer|SetNarrationBool (Subsystems|GetNarrationVariablesContainer) _asactor "TalkToMePrimary" false)
      (Default|UpdateWidget (Actor|GetComponentbyClass _asactor "/Game/_Main/Mechanics/Narration/TalkToMe/BP_TalkToMe.BP_TalkToMe_C"))
      ;[0 0.000581 0.005] Wyspawnuj Kurwe na pietrze
      (bind _returnvalue (Game|SpawnActorfromClass "/Game/_Main/Mechanics/Characters/BP_Ann.BP_Ann_C" (Math|Transform|MakeTransform "877.999997,6523.000000,920.000002" "0.000000,217.946544,0.000000" "1.000000,1.000000,1.000000") "AlwaysSpawn" "MultiplyWithRoot" 0 0))
      (Class|NarrationVariablesContainer|SetNarrationBool (Subsystems|GetNarrationVariablesContainer) _returnvalue "TalkToMePrimary" true)
      (Default|UpdateWidget (Actor|GetComponentbyClass _returnvalue "/Game/_Main/Mechanics/Narration/TalkToMe/BP_TalkToMe.BP_TalkToMe_C"))
      (Class|BPIDetectiveGameInstance|SetHudPrimaryText(Message) (Game|GetGameInstance) "Udaj się do pokoju na piętrze i wyjasnij Ani sytuacje ")
      (Class|BPIDetectiveGameInstance|SetHudTip(Message) (Game|GetGameInstance)))
    (:AnnDialogue0
      (CallFunction|AnnDIalogue0))
    (:AnnDialogue1
      (CallFunction|AnnDialogue1))
    (:BedInteractedWith
      (CallFunction|BedInteractedwith))
    (:RejectedByBegars
      (Class|BPIDetectiveGameInstance|SetHudPrimaryText(Message) (Game|GetGameInstance) "Znajdź sposób na uzyskanie informacji od żebraków")
      (Class|BPIDetectiveGameInstance|SetHudTip(Message) (Game|GetGameInstance) "Żebracy to cwane bestie ale z każdym kolejnym pensem stają się potulniejszymi owieczkami"))))

(event EventSetWorldState
  (Utilities|FlowControl|DelayUntilNextTick)
  (bind _returnvalue (Class|QuestGraph|CurrentWorldIs "/Game/_Main/Levels/City/MainCity/BlockoutCityNat.BlockoutCityNat"))
  (if _returnvalue
    (bind _outcome (Class|QuestGraph|GetObjectiveOutcome "Narration1"))
    (switch name _outcome
      (:None
        ;[0 0.000581 0.005] Odejdz powoli kawalek od drzwi
        (Utilities|MovePlayerto (Game|GetPlayerController 0) (Math|Vector|MakeVector 19.367133 27781.12009 155.000009) 1.5e+02
          (:On%20Success
            _)))
      (:Success
        _))
    (Class|QuestGraph|SetObjectiveOutcome "Narration1" "Success" false)
    (bind _outcome_2 (Class|QuestGraph|GetObjectiveOutcome "FindHostelsInfo"))
    (switch name _outcome_2
      (:None
        ;[0 0.9427 0.9427] Od biura detektywa jest jedna droga powrotna na rynek, pozostałe są zastawione przez np. patrole straży miejskiej.
        (CallFunction|SpawnZapory+StrazMiejska)
        ;[0 1 0.9296] Spawn ulotki
        (CallFunction|EnableLeaflets)
        ;[0 1 0.9792] Spawn ludzi menelaos w parku
        (CallFunction|SpawnBeggars)
        ;[0 0.000581 0.005] Schowaj drzwi do burdelu
        (bind _outactors (Actor|GetAllActorsOfClasswithTag "/Game/_Main/Mechanics/LevelChangeSpot/BP_LevelChangeSpot.BP_LevelChangeSpot_C" "LevelChangerBurdel"))
        (Transformation|SetActorLocation (Utilities|Array|Get(acopy) _outactors) (+ (Transformation|GetActorLocation (Utilities|Array|Get(acopy) _outactors)) "0.000000,0.000000,1000.000000") false false)))
    (else
      (bind _returnvalue_2 (Class|QuestGraph|CurrentWorldIs "/Game/_Main/Levels/ClosedLocations/NewBurdello/MainBurdelloJS.MainBurdelloJS"))
      (if _returnvalue_2
        ;[0 0.000581 0.005] Juz nie bedzie mozna wyjsc z burdelu
        (CallFunction|HideBurdelloDoor)
        (bind _outactors_2 (Actor|GetAllActorswithInterface "/Game/_Main/Mechanics/Characters/BPI_Barman.BPI_Barman_C"))
        (Class|NarrationVariablesContainer|SetNarrationBool (Subsystems|GetNarrationVariablesContainer) (Utilities|Array|Get(acopy) _outactors_2) "TalkToMePrimary" true)
        (Default|UpdateWidget (Actor|GetComponentbyClass (Utilities|Array|Get(acopy) _outactors_2) "/Game/_Main/Mechanics/Narration/TalkToMe/BP_TalkToMe.BP_TalkToMe_C"))))))

(fn GetDefaultQuestData
  (return (Utilities|Struct|MakeGraphQuestData (Utilities|Map|MakeMap "(TagName=\"GraphQuest.ObjectiveText.Title\")" "Quest 2" "(TagName=\"GraphQuest.ObjectiveText.Description\")" "") "(GameplayTags=)" (Class|QuestGraph|AppendObjectives (Utilities|Map|MakeMap "Narration1" (Utilities|Struct|MakeGraphQuestObjective (Utilities|Map|MakeMap "(TagName=\"GraphQuest.ObjectiveText.Title\")" "Narration1") "(GameplayTags=((TagName=\"GraphQuest.ObjectiveParameter.Hidden\")))")) (Class|QuestGraph|AppendObjectives (Utilities|Map|MakeMap "FindSleepingPlace" (Utilities|Struct|MakeGraphQuestObjective (Utilities|Map|MakeMap "(TagName=\"GraphQuest.ObjectiveText.Title\")" "Spędź noc w Manchesterze" "(TagName=\"GraphQuest.ObjectiveText.Description\")" "Spędź noc w Manchesterze") "(GameplayTags=)") "FindHostelsInfo" (Utilities|Struct|MakeGraphQuestObjective (Utilities|Map|MakeMap "(TagName=\"GraphQuest.ObjectiveText.Title\")" "Poszukaj informacji o hostelach na rynku." "(TagName=\"GraphQuest.ObjectiveText.Description\")" "Znajdź sklep i kup mapę miasta.") "(GameplayTags=)") "CoinFound" (Utilities|Struct|MakeGraphQuestObjective (Utilities|Map|MakeMap "(TagName=\"GraphQuest.ObjectiveText.Title\")" "Coin" "(TagName=\"GraphQuest.ObjectiveText.Description\")" "Znajdz coin zeby dac zebrakowi w parku") "(GameplayTags=((TagName=\"GraphQuest.ObjectiveParameter.Hidden\")))") "RejectedByBegars" (Utilities|Struct|MakeGraphQuestObjective (Utilities|Map|MakeMap "(TagName=\"GraphQuest.ObjectiveText.Title\")" "" "(TagName=\"GraphQuest.ObjectiveText.Description\")" "") "(GameplayTags=((TagName=\"GraphQuest.ObjectiveParameter.Hidden\")))")) (Utilities|Map|MakeMap "AnnDialogue0" (Utilities|Struct|MakeGraphQuestObjective (Utilities|Map|MakeMap "(TagName=\"GraphQuest.ObjectiveText.Title\")" "Porozmawiaj z Anią " "(TagName=\"GraphQuest.ObjectiveText.Description\")" "Wytlumacz jej swoją sytuacje") "(GameplayTags=)") "AnnDialogue1" (Utilities|Struct|MakeGraphQuestObjective (Utilities|Map|MakeMap "(TagName=\"GraphQuest.ObjectiveText.Title\")" "Lepiej poznaj Anie" "(TagName=\"GraphQuest.ObjectiveText.Description\")" "ASwda") "(GameplayTags=)")))))))

(fn SpawnZapory+StrazMiejska
  (Utilities|FlowControl|Sequence
    (:then_0
      ;[0 0.000581 0.005] Gates
      (bind _outactors (Actor|GetAllActorsOfClasswithTag "/Game/_Main/Art/Props/Wall/BP_Gate.BP_Gate_C" "GateShop0"))
      (Default|SetOpen (Utilities|Array|Get(acopy) _outactors) false)
      (bind _outactors_2 (Actor|GetAllActorsOfClasswithTag "/Game/_Main/Art/Props/Wall/BP_Gate.BP_Gate_C" "GateShop1"))
      (Default|SetOpen (Utilities|Array|Get(acopy) _outactors_2) false)
      (bind _outactors_3 (Actor|GetAllActorsOfClasswithTag "/Game/_Main/Art/Props/Wall/BP_Gate.BP_Gate_C" "GatePark0"))
      (Default|SetOpen (Utilities|Array|Get(acopy) _outactors_3) true))
    (:then_1
      (for _array_element (LocalVariables|GetOfficersLocations)
        (bind _returnvalue (Game|SpawnActorfromClass "/Game/_Main/Mechanics/Characters/BP_OfficerQuest2.BP_OfficerQuest2_C" _array_element "AlwaysSpawn" "MultiplyWithRoot" 0 0))
        (Class|NarrationVariablesContainer|SetNarrationBool (Subsystems|GetNarrationVariablesContainer) _returnvalue "TalkToMe" true)
        (Default|UpdateWidget (Actor|GetComponentbyClass _returnvalue "/Game/_Main/Mechanics/Narration/TalkToMe/BP_TalkToMe.BP_TalkToMe_C"))))))

(fn EnableLeaflets
  (bind _outactors (Actor|GetAllActorsOfClass "/Game/_Main/Mechanics/Quests/QuestProps/BP_leafletProp.BP_leafletProp_C"))
  (for _array_element _outactors
    (Collision|SetCollisionEnabled (Variables|/Game/_Main/Mechanics/Quests/QuestProps/BP_leafletProp.BP_leafletProp_C|GetRangeArea _array_element) "QueryOnly")))

(fn SpawnBeggars
  (bind _returnvalue (Game|SpawnActorfromClass "/Game/_Main/Mechanics/Characters/BP_BeggarTalkableQuest2.BP_BeggarTalkableQuest2_C" (Math|Transform|MakeTransform "5740.000000,27670.000000,160.000000" "0.000000,10.000000,0.000000" "1.000000,1.000000,1.000000") "AlwaysSpawn" "MultiplyWithRoot" 0 0))
  (Class|NarrationVariablesContainer|SetNarrationBool (Subsystems|GetNarrationVariablesContainer) _returnvalue "TalkToMePrimary" true)
  (Default|UpdateWidget (Actor|GetComponentbyClass _returnvalue "/Game/_Main/Mechanics/Narration/TalkToMe/BP_TalkToMe.BP_TalkToMe_C"))
  (Game|SpawnActorfromClass "/Game/_Main/Mechanics/Characters/BP_BeggarQuest2.BP_BeggarQuest2_C" (Math|Transform|MakeTransform "5930.000000,27700.000000,160.000000" "0.000000,169.999999,0.000000" "1.000000,1.000000,1.000000") "AlwaysSpawn" "MultiplyWithRoot" 0 0))

(fn SpawnCoin
  (bind _returnvalue (Game|SpawnActorfromClass "/Game/_Main/Mechanics/Quests/QuestProps/BP_CoinQuest2.BP_CoinQuest2_C" (Math|Transform|MakeTransform "6680.000000,27980.000000,80.000000" "0, 0, 0" "1.000000,1.000000,1.000000") "Undefined" "MultiplyWithRoot" 0 0))
  (Variables|/Game/_Main/Mechanics/Quests/QuestProps/BP_CoinQuest2.BP_CoinQuest2_C|SetID _returnvalue "CoinFound")
  (Collision|SetCollisionEnabled (Variables|/Game/_Main/Mechanics/Quests/QuestProps/BP_CoinQuest2.BP_CoinQuest2_C|GetRangeArea _returnvalue) "QueryOnly"))

(fn HideBurdelloDoor
  (bind _outactors (Actor|GetAllActorsOfClasswithTag "/Game/_Main/Mechanics/LevelChangeSpot/BP_LevelChangeSpot.BP_LevelChangeSpot_C" "LevelChangerBurdelInside"))
  (CallFunction|SetGameTime 21)
  (Class|BPIDetectiveGameInstance|SetHudPrimaryText(Message) (Game|GetGameInstance) "Porozmawiaj z Barmanem")
  (Class|BPIDetectiveGameInstance|SetHudTip(Message) (Game|GetGameInstance))
  (Transformation|SetActorLocation (Utilities|Array|Get(acopy) _outactors) (+ (Transformation|GetActorLocation (Utilities|Array|Get(acopy) _outactors)) "0.000000,0.000000,-1000.000000") false false))